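; Openable door actor that swings open and closed in response to OpenDoor events.
; It stores its rotation at BeginPlay, and the DoorSwing timeline adds an animated yaw offset to it while opening, or plays in reverse to close.
; A Sound Timing event track on the timeline plays the door lock sound at the actor's location.
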(event `self.ReceiveBeginPlay`
  (set `self.initialRotation` (`self.K2_GetActorRotation`)))

(event `self.OpenDoor.OnOpen`
  (bind (_direction _openangle) (`Timeline|Door Swing` :!label _label)
    (:`Update`
      (`self.K2_SetActorRotation` (`KismetMathLibrary.ComposeRotators` (`KismetMathLibrary.MakeRotator` 0.0 0.0 _openangle) (`self.initialRotation`))))
    (:`Sound Timing`
      (`GameplayStatics.PlaySoundAtLocation` "/Game/Sounds/door_lock.door_lock" (`self.K2_GetActorLocation`) (struct) 1.0 1.0 0.0 null null null))))

(event `self.OpenDoor.OnClose`
  (goto _label :!via `Reverse`))

(fn `UserConstructionScript`)